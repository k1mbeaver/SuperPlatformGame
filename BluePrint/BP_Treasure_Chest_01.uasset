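; Treasure chest actor that swings its lid open when the player character overlaps it and closes it when they leave.
; Begin and end overlap events play and reverse the Lid_Open timeline, whose LidOpen track scales the lid's relative rotation up to 120 degrees.
; The construction script applies the TreasureMaterial variable to the base, lid and treasure meshes.
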(event Custom|OpenChest
  (bind _lidopen (Timeline|Lid_Open Play)
    (:Update
      (Transformation|SetRelativeRotation (Variables|Default|GetLid) (* "0, 0,-120.000000" _lidopen) false false))))

(event Custom|ClosedChest
  (bind _lidopen (Timeline|Lid_Open Reverse)
    (:Update
      (Transformation|SetRelativeRotation (Variables|Default|GetLid) (* "0, 0,-120.000000" _lidopen) false false))))

(event EventBeginPlay)

(event Collision|EventActorBeginOverlap
  (params (OtherActor :type Actor%20Object%20Reference))
  (if (== OtherActor (Game|GetPlayerCharacter 0))
    (CallFunction|OpenChest)))

(event EventTick
  (params (DeltaSeconds :type Float%20%28single-precision%29)))

(event Collision|EventActorEndOverlap
  (params (OtherActor :type Actor%20Object%20Reference))
  (if (== OtherActor (Game|GetPlayerCharacter 0))
    (CallFunction|ClosedChest)))

(fn ConstructionScript
  (bind _treasure_material (Variables|Default|GetTreasure%20Material))
  (Rendering|Material|SetMaterial (Variables|Default|GetBase) 0 _treasure_material)
  (Rendering|Material|SetMaterial (Variables|Default|GetTreasure) 0 _treasure_material))